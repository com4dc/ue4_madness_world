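; TongariCone is an actor, apparently a cone, that stretches vertically when another actor overlaps it.
; The first timeline blends its scale toward ten times height while keeping location and rotation.
; When that finishes and Universe is true, a second timeline moves it upward.
; Both lerps start from the current transform each update, so the motion compounds rather than following a fixed start-to-end path.
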(event EventBeginPlay)

(event EventActorBeginOverlap
  (params (OtherActor :type Actor%20Object%20Reference))
  (bind _returnvalue (Transformation|GetActorLocation))
  (bind _新規track_1 (Timeline|タイムライン_0 PlayFromStart)
    (:Update
      (Transformation|SetActorTransform (Math|Transform|Lerp(Transform) (Transformation|GetActorTransform) (Math|Transform|MakeTransform _returnvalue (Transformation|GetActorRotation) "1.000000,1.000000,10.000000") _新規track_1)))
    (:Finished
      (if (Variables|Default|Getuniverse)
        (bind _新規track_2 (Timeline|タイムライン_1 PlayFromStart)
          (:Update
            (Transformation|SetActorLocationAndRotation (Math|Vector|Lerp(Vector) _returnvalue (+ _returnvalue "0, 0,1000.000000") _新規track_2) "0, 0, 0")))))))

(event EventTick
  (params (DeltaSeconds :type Float%20%28single-precision%29)))

(fn ConstructionScript)