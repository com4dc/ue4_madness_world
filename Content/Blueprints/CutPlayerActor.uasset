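; CutPlayerActor is a moving-wall obstacle whose two walls slide toward each other and back, with no damage or overlap logic in this graph.
; The construction script spaces the walls along the actor's right vector by DistanceBetweenWalls.
; At BeginPlay it caches endpoints from WallMoveLength, scales timeline speed by CloseCycle and starts a looping timer.
; Each tick of that timer restarts the Moving timeline, which lerps both walls and reverses on finish.
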(event Custom|move
  ;[1 1 1] setTimerで指定した時間間隔分で移動する
  (bind _alpha (Timeline|moving PlayFromStart)
    (:Update
      (Transformation|SetWorldLocation (Variables|Default|Getwall1) (Math|Vector|Lerp(Vector) (Variables|Default|GetDefaultPosition_L) (Variables|Default|GetDesiredPosition_L) _alpha) false false)
      (Transformation|SetWorldLocation (Variables|Default|Getwall2) (Math|Vector|Lerp(Vector) (Variables|Default|GetDefaultPosition_R) (Variables|Default|GetDesiredPosition_R) _alpha) false false))
    (:Finished
      (CallFunction|Back))))

(event Custom|back
  ;[1 1 1] setTimerで指定した時間間隔分で移動する
  (bind _alpha (Timeline|moving ReverseFromEnd)
    (:Update
      (Transformation|SetWorldLocation (Variables|Default|Getwall1) (Math|Vector|Lerp(Vector) (Variables|Default|GetDefaultPosition_L) (Variables|Default|GetDesiredPosition_L) _alpha) false false)
      (Transformation|SetWorldLocation (Variables|Default|Getwall2) (Math|Vector|Lerp(Vector) (Variables|Default|GetDefaultPosition_R) (Variables|Default|GetDesiredPosition_R) _alpha) false false))
    (:Finished
      (CallFunction|Back))))

(event EventBeginPlay
  (bind _returnvalue (Transformation|GetActorRightVector))
  (bind _closecycle (Variables|Default|GetCloseCycle))
  (bind _wallmovelength (Variables|Default|GetWallMoveLength))
  (bind _returnvalue_2 (* _returnvalue _wallmovelength))
  (Utilities|FlowControl|Sequence
    (:then_0
      ;[1 1 1] 今の壁の位置とWallMoveLength分だけ移動した時の位置を保存
      (bind _output_get (Variables|Default|SetDefaultPosition_L (Transformation|GetWorldLocation (Variables|Default|Getwall1))))
      (Variables|Default|SetDesiredPosition_L (+ _output_get _returnvalue_2)))
    (:then_1
      (bind _output_get_2 (Variables|Default|SetDefaultPosition_R (Transformation|GetWorldLocation (Variables|Default|Getwall2))))
      (Variables|Default|SetDesiredPosition_R (- _output_get_2 _returnvalue_2)))
    (:then_2
      (Components|Timeline|SetPlayRate (Variables|Default|Getmoving) (/ 1.0 _closecycle))
      (Utilities|Time|SetTimerbyEvent (delegate Custom|move) (* 0.4 _closecycle) true))))

(event EventActorBeginOverlap
  (params (OtherActor :type Actor%20Object%20Reference)))

(event EventTick
  (params (DeltaSeconds :type Float%20%28single-precision%29)))

(fn ConstructionScript
  (bind _wall1 (Variables|Default|Getwall1))
  (bind _wall2 (Variables|Default|Getwall2))
  ;[1 1 1] 壁の初期位置を決める
  (Transformation|SetWorldLocation _wall1 (+ (Transformation|GetWorldLocation _wall1) (* (* (Transformation|GetActorRightVector) (/ (Variables|Default|GetDistanceBetweenWalls) 2.0)) -1.0)) false false)
  (Transformation|SetWorldLocation _wall2 (+ (Transformation|GetWorldLocation _wall2) (* (Transformation|GetActorRightVector) (/ (Variables|Default|GetDistanceBetweenWalls) 2.0))) false false))