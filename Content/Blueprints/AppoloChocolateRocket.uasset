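; Apollo chocolate rocket actor that launches itself on BeginPlay and then removes itself.
; A first timeline spins it and stretches its Z scale in place, then a second moves it toward a fixed world point high above the origin.
; Both lerp from the current transform each update rather than a stored start.
; When the flight finishes, a particle system runs briefly and switches off before the actor is destroyed after another delay.
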(event EventBeginPlay
  (bind _returnvalue (Transformation|GetActorTransform))
  (bind _particlesystem (Variables|Default|GetParticleSystem))
  (bind _kaiten (Timeline|初期回転 PlayFromStart)
    (:Update
      (Transformation|SetActorTransform (Math|Transform|Lerp(Transform) _returnvalue (Math|Transform|MakeTransform (.Location (Math|Transform|BreakTransform _returnvalue)) (Math|Rotator|Lerp(Rotator) (Transformation|GetActorRotation) "0,360.000000, 0" _kaiten) "1,1,100.000000") _kaiten)))
    (:Finished
      (bind _新規track_2 (Timeline|飛ぶ PlayFromStart)
        (:Update
          (Transformation|SetActorLocationAndRotation (Math|Vector|Lerp(Vector) (Transformation|GetActorLocation) "0, 0,5000.000000" _新規track_2) (Math|Rotator|Lerp(Rotator) (Transformation|GetActorRotation) "0,360.000000, 0" _新規track_2)))
        (:Finished
          (Components|Activation|Activate _particlesystem false)
          (Utilities|FlowControl|Delay 5.0)
          (Components|Activation|Deactivate _particlesystem)
          (Utilities|FlowControl|Delay 5.0)
          (Actor|DestroyActor))))))

(event EventActorBeginOverlap
  (params (OtherActor :type Actor%20Object%20Reference)))

(event EventTick
  (params (DeltaSeconds :type Float%20%28single-precision%29)))

(fn ConstructionScript)